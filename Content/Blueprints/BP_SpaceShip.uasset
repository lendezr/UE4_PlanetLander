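; Player-controlled physics spaceship with roll, pitch, yaw, forward and vertical thrust, and a toggle between cockpit and external cameras.
; Rotation inputs drive paired thruster components, while engine inputs apply impulses to the ship mesh along the direction arrow.
; Forward thrust requires fuel and schedules its depletion by timer; vertical thrust ignores fuel.
; Tick tints both engines' dynamic materials from grey to green using summed velocity components.
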(event Custom|DepleteFuel
  ;[1 1 1] Handles moving forward
  (Variables|Default|SetcurrentFuel (- (Variables|Default|GetcurrentFuel) (Variables|Default|GetdepletionRate))))

(event EventTick
  (params (DeltaSeconds :type Float%20%28single-precision%29))
  (bind _shipmesh (Variables|Default|GetShipMesh))
  (bind _returnvalue (Transformation|GetComponentVelocity _shipmesh))
  (bind _returnvalue_2 (+ (.x _returnvalue) (.y _returnvalue) (.z _returnvalue)))
  (bind _returnvalue_3 (/ _returnvalue_2 5e+03))
  (bind _returnvalue_4 (Math|Float|Absolute(Float) _returnvalue_3))
  (bind _returnvalue_5 (Math|Color|Lerp(LinearColor) "(R=0.255208,G=0.255208,B=0.255208,A=1.000000)" "(R=0.094678,G=1.000000,B=0.000000,A=1.000000)" _returnvalue_4))
  (Rendering|Material|SetVectorParameterValue (Variables|Default|GetMD_engineR) "thrust" _returnvalue_5 :!class /Script/Engine.MaterialInstanceDynamic)
  (Rendering|Material|SetVectorParameterValue (Variables|Default|GetMD_engineL) "thrust" _returnvalue_5 :!class /Script/Engine.MaterialInstanceDynamic))

(event EventBeginPlay
  (bind _returnvalue (Rendering|Material|CreateDynamicMaterialInstance (Variables|Default|GetEngineR) 0 "/Game/Materials/Mi_engineThrust.Mi_engineThrust" "None" :!class /Script/Engine.PrimitiveComponent))
  (Variables|Default|SetMD_engineR _returnvalue)
  (bind _returnvalue_2 (Rendering|Material|CreateDynamicMaterialInstance (Variables|Default|GetEngineL) 0 "/Game/Materials/Mi_engineThrust.Mi_engineThrust" "None" :!class /Script/Engine.PrimitiveComponent))
  (Variables|Default|SetMD_engineL _returnvalue_2))

(event Input|ActionEvents|InputActionToggleCameraView
  (params (Key :type Key%20Structure))
  (bind _cockpitcamera (Variables|Default|GetCockpitCamera))
  (bind _externalcamera (Variables|Default|GetExternalCamera))
  ;[1 1 1] Handels switching between external and cockpit views
  (:Pressed
    (Utilities|FlowControl|FlipFlop
      (:A
        (Components|Activation|Activate _cockpitcamera false)
        (Components|Activation|Deactivate _externalcamera))
      (:B
        (Components|Activation|Activate _externalcamera false)
        (Components|Activation|Deactivate _cockpitcamera)))))

(event Input|AxisEvents|InputAxisEngineThrust
  (params (AxisValue :type Float%20%28single-precision%29))
  ;[1 1 1] Handles moving forward
  (if (not (<= (Variables|Default|GetcurrentFuel) 0.0))
    (Physics|AddImpulse (Variables|Default|GetShipMesh) (* (Math|Vector|GetForwardVector (Transformation|GetWorldRotation (Variables|Default|GetRootDirectionArrow))) (* AxisValue (Variables|Default|GetEnginePower))) "None" false)
    (Utilities|Time|SetTimerbyEvent (delegate Custom|DepleteFuel) 0.05)))

(event Input|AxisEvents|InputAxisRoll
  (params (AxisValue :type Float%20%28single-precision%29))
  (bind _rightwingrollthrust (Variables|Default|GetRightWingRollThrust))
  (bind _rollstrenght (Variables|Default|GetRollStrenght))
  (bind _leftwingrollthrust (Variables|Default|GetLeftWingRollThrust))
  (bind _returnvalue (* AxisValue _rollstrenght))
  ;[1 1 1] Handles Rolling
  (if (!= AxisValue 0.0)
    (Variables|/Script/Engine.PhysicsThrusterComponent|SetThrustStrength _leftwingrollthrust _returnvalue)
    (Variables|/Script/Engine.PhysicsThrusterComponent|SetThrustStrength _rightwingrollthrust _returnvalue)
    (Components|Activation|Activate _leftwingrollthrust false)
    (Components|Activation|Activate _rightwingrollthrust false)
    (else
      (Components|Activation|Deactivate (Variables|Default|GetLeftWingRollThrust))
      (Components|Activation|Deactivate (Variables|Default|GetRightWingRollThrust)))))

(event Input|AxisEvents|InputAxisEngineThrustUp
  (params (AxisValue :type Float%20%28single-precision%29))
  ;[1 1 1] Handles moving upwards
  (Physics|AddImpulse (Variables|Default|GetShipMesh) (* (Math|Vector|GetUpVector (Transformation|GetWorldRotation (Variables|Default|GetRootDirectionArrow))) (* AxisValue (Variables|Default|GetEnginePower))) "None" false))

(event Input|AxisEvents|InputAxisPitch
  (params (AxisValue :type Float%20%28single-precision%29))
  (bind _nosepitchthruster (Variables|Default|GetNosePitchThruster))
  (bind _tailpitchthruster (Variables|Default|GetTailPitchThruster))
  (bind _pitchstrenght (Variables|Default|GetPitchStrenght))
  (bind _returnvalue (* AxisValue _pitchstrenght))
  ;[1 1 1] Handles Pitching
  (if (!= AxisValue 0.0)
    (Variables|/Script/Engine.PhysicsThrusterComponent|SetThrustStrength _nosepitchthruster _returnvalue)
    (Variables|/Script/Engine.PhysicsThrusterComponent|SetThrustStrength _tailpitchthruster _returnvalue)
    (Components|Activation|Activate _nosepitchthruster false)
    (Components|Activation|Activate _tailpitchthruster false)
    (else
      (Components|Activation|Deactivate (Variables|Default|GetNosePitchThruster))
      (Components|Activation|Deactivate (Variables|Default|GetTailPitchThruster)))))

(event Input|AxisEvents|InputAxisYaw
  (params (AxisValue :type Float%20%28single-precision%29))
  (bind _yawstrenght (Variables|Default|GetYawStrenght))
  (bind _noseyawthrust (Variables|Default|GetNoseYawThrust))
  (bind _tailyawthrust (Variables|Default|GetTailYawThrust))
  (bind _returnvalue (* AxisValue _yawstrenght))
  ;[1 1 1] Handles Yawing
  (if (!= AxisValue 0.0)
    (Variables|/Script/Engine.PhysicsThrusterComponent|SetThrustStrength _noseyawthrust _returnvalue)
    (Variables|/Script/Engine.PhysicsThrusterComponent|SetThrustStrength _tailyawthrust _returnvalue)
    (Components|Activation|Activate _noseyawthrust false)
    (Components|Activation|Activate _tailyawthrust false)
    (else
      (Components|Activation|Deactivate (Variables|Default|GetNoseYawThrust))
      (Components|Activation|Deactivate (Variables|Default|GetTailYawThrust)))))

(fn ConstructionScript)